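; BP_PlayerCharacter is the player character Blueprint, handling movement, look and jump through Turkish-named input mappings.
; Forward and strafe axes feed AddMovementInput using vectors from a zero rotator, so movement follows fixed world axes rather than the view.
; Look axes drive controller yaw and pitch, and Zipla starts and stops jumping.
; The EtkilesimYap interact action only clears EtkilesimHedefi, and a PlayerStart cast is left unconnected.
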(event `InputAxis|IleriGeri`
  (params (AxisValue :type "Float (single-precision)"))
  (`self.AddMovementInput` (`KismetMathLibrary.GetForwardVector` (struct)) AxisValue))

(event `InputAxis|YanaBak`
  (params (AxisValue :type "Float (single-precision)"))
  (`self.AddControllerYawInput` AxisValue))

(event `InputAxis|YukariAsagiBak`
  (params (AxisValue :type "Float (single-precision)"))
  (`self.AddControllerPitchInput` AxisValue))

(event `InputAxis|SagaSola`
  (params (AxisValue :type "Float (single-precision)"))
  (`self.AddMovementInput` (`KismetMathLibrary.GetRightVector` (struct)) AxisValue))

(event `InputAction|EtkilesimYap`
  (params (Key :type "Key Structure"))
  (:`Pressed`
    (set `self.EtkilesimHedefi` null)))

(event `InputAction|Zipla`
  (params (Key :type "Key Structure"))
  (:`Pressed`
    (`self.Jump`))
  (:`Released`
    (`self.StopJumping`)))

(fn `UserConstructionScript`)